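; Item pickup trigger for the kart game that gives an overlapping player or AI kart one of five random power-ups.
; On overlap it calls Interaction, then sets the kart's ReceivedPowerUpNb to the random roll.
; Player karts also receive a new Item_WID_HUD showing the matching icon, with a pickup sound played at world origin.
; An older HUD cleanup and viewport chain is left disconnected.
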(event `self.ReceiveActorBeginOverlap`
  (params (OtherActor :type "Actor Object Reference"))
  (bind _itemhudref (`self.ItemHUDRef`))
  (bind _pawnref (`self.PawnRef`))
  (bind _itemhudref_2 (`self.ItemHUDRef`))
  (bind _aipawnref (`self.AIPawnRef`))
  (bind _pawnref_2 (`self.PawnRef`))
  (`|ExecutionSequence`
    (:`then_0`
      ;[1 1 1] GetRerefence
      (bind _asbp_kart_pawn_base_child (cast `/Game/KIA_Game/template/template_BP/BP_KartPawnBase_Child` OtherActor))
      (set `self.PawnRef` _asbp_kart_pawn_base_child)
      (`self.Interaction`)
      (bind _returnvalue (`|CreateWidget` "/Game/KIA_Game/Game_BP/PowerUpDown/Item_WID_HUD.Item_WID_HUD_C"))
      (bind _output_get (set `self.ItemHUDRef` _returnvalue))
      (`/Game/KIA_Game/template/template_BP/BP_KartPawnBase_Child.SetNewHUD` (`self.PawnRef`) _output_get)
      ;[1 1 1] GiveItemToOverlapingActor
      (switch `int` (+ (`KismetMathLibrary.RandomInteger` 5) 1)
        (:`1`
          (set `/Game/KIA_Game/template/template_BP/BP_KartPawnBase.Received Power Up Nb` 1 _pawnref_2)
          ;[1 1 1] ChangeIconForHUD
          (bind _output_get_2 (set `self.DefaultPowerUpIcon` (`self.PowerUpBombIcon`)))
          (`/Game/KIA_Game/Game_BP/PowerUpDown/Item_WID_HUD.GetIcon` _itemhudref_2 _output_get_2))
        (:`2`
          (set `/Game/KIA_Game/template/template_BP/BP_KartPawnBase.Received Power Up Nb` 2 _pawnref_2)
          (bind _output_get_3 (set `self.DefaultPowerUpIcon` (`self.PowerUpBoostIcon`)))
          (`/Game/KIA_Game/Game_BP/PowerUpDown/Item_WID_HUD.GetIcon` _itemhudref_2 _output_get_3))
        (:`3`
          (set `/Game/KIA_Game/template/template_BP/BP_KartPawnBase.Received Power Up Nb` 3 _pawnref)
          (bind _output_get_4 (set `self.DefaultPowerUpIcon` (`self.PowerUpReverseZoneIcon`)))
          (`/Game/KIA_Game/Game_BP/PowerUpDown/Item_WID_HUD.GetIcon` _itemhudref _output_get_4))
        (:`4`
          (set `/Game/KIA_Game/template/template_BP/BP_KartPawnBase.Received Power Up Nb` 4 _pawnref)
          (bind _output_get_5 (set `self.DefaultPowerUpIcon` (`self.PowerUpGrow`)))
          (`/Game/KIA_Game/Game_BP/PowerUpDown/Item_WID_HUD.GetIcon` _itemhudref _output_get_5))
        (:`5`
          (set `/Game/KIA_Game/template/template_BP/BP_KartPawnBase.Received Power Up Nb` 5 _pawnref)
          (bind _output_get_6 (set `self.DefaultPowerUpIcon` (`self.PowerUpFastForward`)))
          (`/Game/KIA_Game/Game_BP/PowerUpDown/Item_WID_HUD.GetIcon` _itemhudref _output_get_6)))
      (`GameplayStatics.PlaySoundAtLocation` "/Game/KIA_Game/audio/PowerUp/PickUpPowerUpSound.PickUpPowerUpSound" (0.0 0.0 0.0) (struct) 1.0 1.0 0.0 null null null))
    (:`then_1`
      (bind _asbp_kart_pawn_base_ai_temp (cast `/Game/KIA_Game/template/template_BP/BasicAI/BP_KartPawnBase_AiTemp` OtherActor))
      (set `self.AIPawnRef` _asbp_kart_pawn_base_ai_temp)
      (`self.Interaction`)
      (switch `int` (+ (`KismetMathLibrary.RandomInteger` 5) 1)
        (:`1`
          (set `/Game/KIA_Game/template/template_BP/BP_KartPawnBase.Received Power Up Nb` 1 _aipawnref))
        (:`2`
          (set `/Game/KIA_Game/template/template_BP/BP_KartPawnBase.Received Power Up Nb` 2 _aipawnref))
        (:`3`
          (set `/Game/KIA_Game/template/template_BP/BP_KartPawnBase.Received Power Up Nb` 3 _aipawnref))
        (:`4`
          (set `/Game/KIA_Game/template/template_BP/BP_KartPawnBase.Received Power Up Nb` 4 _aipawnref))
        (:`5`
          (set `/Game/KIA_Game/template/template_BP/BP_KartPawnBase.Received Power Up Nb` 5 _aipawnref))))))

(fn `UserConstructionScript`)