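; BP_ItemSpawner is an actor that spawns a random item at its own location and keeps one current item at a time.
; On BeginPlay it spawns a scaled-up pick from ItemsToSpawn, sets itself as Owner and stores it as CurrentItem.
; A Respawn event clears that reference, waits SpawnDelay, then spawns again only if no valid item is held.
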(event `self.ReceiveBeginPlay`
  (`self.AttemptToSpawn`))

(event `/Game/KIA_Game/Game_BP/PowerUpDown/BPI_ItemSpawner.Respawn`
  (set `self.CurrentItem` null)
  (`KismetSystemLibrary.Delay` (`self.SpawnDelay`))
  (`self.AttemptToSpawn`))

(fn `AttemptToSpawn`
  (`/Engine/EditorBlueprintResources/StandardMacros.IsValid` (`self.CurrentItem`)
    (:`Is Not Valid`
      (`self.SpawnItem`))))

(fn `SpawnItem`
  (bind _returnvalue (`|SpawnActorFromClass` (`|GetArrayItem` (`self.ItemsToSpawn`) (`KismetMathLibrary.RandomIntegerInRange` 0 (- (`KismetArrayLibrary.Array_Length` (`self.ItemsToSpawn`)) 1))) (`KismetMathLibrary.MakeTransform` (`self.K2_GetActorLocation`) (`self.K2_GetActorRotation`) (1.5 1.5 1.5)) "Undefined" "OverrideRootScale" self null))
  (set `self.CurrentItem` _returnvalue))

(fn `UserConstructionScript`)