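; Bouncing kart power-up projectile in the style of a green shell, which spins and slows the karts it hits.
; Each tick a downward line trace snaps it to a fixed height above the ground.
; Projectile bounces call SpinAndSlow on player or AI karts without destroying the shell, and count any other hit as a wall.
; It destroys itself on the third wall hit or when its lifetime timer expires.
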(event `self.ReceiveBeginPlay`
  (`KismetSystemLibrary.K2_SetTimerDelegate` (delegate `Destroy`) 8.0))

(event `Destroy`
  (`self.K2_DestroyActor`))

(event `self.ReceiveTick`
  (params (DeltaSeconds :type "Float (single-precision)"))
  (bind _projectile (`self.Projectile`))
  (bind _returnvalue (`SceneComponent.K2_GetComponentLocation` (`self.Projectile`)))
  (bind (_returnvalue_x _returnvalue_y) (`KismetMathLibrary.BreakVector` (`SceneComponent.K2_GetComponentLocation` _projectile)))
  (bind _outhit (`KismetSystemLibrary.LineTraceSingleForObjects` :`Start` _returnvalue :`End` (+ _returnvalue (0.0 0.0 -500.0)) :`ObjectTypes` (`self.Object Types`) :`DrawDebugType` "ForOneFrame"))
  (`SceneComponent.K2_SetWorldLocation` _projectile (`KismetMathLibrary.MakeVector` _returnvalue_x _returnvalue_y (+ (.z (`.Location` (`GameplayStatics.BreakHitResult` _outhit))) 60.0)) false false))

(event `self.ProjectileMovement.OnProjectileBounce`
  (params (ImpactResult :type "HitResult Structure (by ref)") (ImpactVelocity :type "Vector Structure (by ref)"))
  (bind (_bblockinghit _binitialoverlap _time _distance _location _impactpoint _normal _impactnormal _physmat _hitactor) (`GameplayStatics.BreakHitResult` ImpactResult))
  (bind _asbp_kart_pawn_base_child (cast `/Game/KIA_Game/template/template_BP/BP_KartPawnBase_Child` _hitactor)
    (:`then`
      (`/Game/KIA_Game/template/template_BP/BP_KartPawnBase.SpinAndSlow` _asbp_kart_pawn_base_child)
      (`KismetSystemLibrary.PrintString` "hit"))
    (:`CastFailed`
      (bind _asbp_kart_pawn_base_ai_temp (cast `/Game/KIA_Game/template/template_BP/BasicAI/BP_KartPawnBase_AiTemp` _hitactor)
        (:`then`
          (`/Game/KIA_Game/template/template_BP/BP_KartPawnBase.SpinAndSlow` _asbp_kart_pawn_base_ai_temp)
          (`KismetSystemLibrary.PrintString` "Hit AI"))
        (:`CastFailed`
          (bind _result (`/Engine/EditorBlueprintResources/StandardMacros.IncrementInt` (`self.WallHitCount`))
            (:`  `
              (if (== _result 3)
                (`self.K2_DestroyActor`)))))))))

(fn `UserConstructionScript`)