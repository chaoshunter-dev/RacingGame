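; Red-shell-style power-up projectile that travels the track by following the AI spline path, with no targeting or hit logic in its graphs.
; On BeginPlay it takes the first BP_AISplinePathActor found and runs a timeline, rate-scaled by Duration, to set actor location and rotation from spline start to end.
; Each Tick, a downward object trace repositions the Projectile component at a fixed hover height above the traced surface.
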(event `self.ReceiveTick`
  (params (DeltaSeconds :type "Float (single-precision)"))
  (bind _projectile (`self.Projectile`))
  (bind (_returnvalue_x _returnvalue_y) (`KismetMathLibrary.BreakVector` (`SceneComponent.K2_GetComponentLocation` _projectile)))
  (bind _returnvalue (`SceneComponent.K2_GetComponentLocation` (`self.Projectile`)))
  (bind _outhit (`KismetSystemLibrary.LineTraceSingleForObjects` :`Start` _returnvalue :`End` (+ _returnvalue (0.0 0.0 -500.0)) :`ObjectTypes` (`self.Object Types`) :`DrawDebugType` "ForOneFrame"))
  (`SceneComponent.K2_SetWorldLocation` _projectile (`KismetMathLibrary.MakeVector` _returnvalue_x _returnvalue_y (+ (.z (`.Location` (`GameplayStatics.BreakHitResult` _outhit))) 60.0)) false false))

(event `self.ReceiveBeginPlay`
  (bind _spline (`/Game/KIA_Game/template/template_BP/BasicAI/BP_AISplinePathActor.Spline` (`self.SplineRef`)))
  (bind _returnvalue (`KismetMathLibrary.Lerp` 0.0 (`SplineComponent.GetSplineLength` _spline) (`self.Shell Movement Track`)))
  (bind _outactors (`GameplayStatics.GetAllActorsOfClass` "/Game/KIA_Game/template/template_BP/BasicAI/BP_AISplinePathActor.BP_AISplinePathActor_C"))
  (set `self.SplineRef` (`|GetArrayItem` _outactors))
  (`TimelineComponent.SetPlayRate` (`self.Timeline_0`) (/ 1.0 (`self.Duration`)))
  (bind (_direction _shellmovementtrack) (`Timeline|Timeline_0`)
    (:`Update`
      (set `self.Shell Movement Track` _shellmovementtrack)
      (`self.K2_SetActorLocationAndRotation` (`SplineComponent.GetLocationAtDistanceAlongSpline` _spline _returnvalue "World") (`SplineComponent.GetRotationAtDistanceAlongSpline` _spline _returnvalue "World")))))

(fn `UserConstructionScript`)