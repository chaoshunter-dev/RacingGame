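; BP_PowerDownTrigger is a kart pickup that applies a random power-down to the player or AI kart that overlaps it.
; On overlap, separate sequence branches cast to the player and AI kart classes, store the pawn and call Interaction, labeled as self-destruction.
; A random roll then triggers shrink (only at normal size), forced reverse or teleport on that kart.
; The logic is duplicated for each kart class.
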(event `self.ReceiveActorBeginOverlap`
  (params (OtherActor :type "Actor Object Reference"))
  (bind _pawnref (`self.PawnRef`))
  (bind _aipawnref (`self.AIPawnRef`))
  (`|ExecutionSequence`
    (:`then_0`
      ;[1 1 1] GetRerefence
      (bind _asbp_kart_pawn_base_child (cast `/Game/KIA_Game/template/template_BP/BP_KartPawnBase_Child` OtherActor))
      (set `self.PawnRef` _asbp_kart_pawn_base_child)
      ;[1 1 1] DestroySelf
      (`self.Interaction`)
      ;[1 1 1] ActivatePowerDownOnOverlapingActor
      (switch `int` (+ (`KismetMathLibrary.RandomInteger` 3) 1)
        (:`1`
          (if (`/Game/KIA_Game/template/template_BP/BP_KartPawnBase.NormalSize` _pawnref)
            (`/Game/KIA_Game/template/template_BP/BP_KartPawnBase.Shrink` _pawnref)))
        (:`2`
          (`/Game/KIA_Game/template/template_BP/BP_KartPawnBase.ForcedReverse` _pawnref (0.0 0.0 0.0)))
        (:`3`
          (`/Game/KIA_Game/template/template_BP/BP_KartPawnBase.UseTeleport` _pawnref))))
    (:`then_1`
      (bind _asbp_kart_pawn_base_ai_temp (cast `/Game/KIA_Game/template/template_BP/BasicAI/BP_KartPawnBase_AiTemp` OtherActor))
      (set `self.AIPawnRef` _asbp_kart_pawn_base_ai_temp)
      (`self.Interaction`)
      (switch `int` (+ (`KismetMathLibrary.RandomInteger` 3) 1)
        (:`1`
          (if (`/Game/KIA_Game/template/template_BP/BP_KartPawnBase.NormalSize` _aipawnref)
            (`/Game/KIA_Game/template/template_BP/BP_KartPawnBase.Shrink` _aipawnref)))
        (:`2`
          (`/Game/KIA_Game/template/template_BP/BP_KartPawnBase.ForcedReverse` _aipawnref (0.0 0.0 0.0)))
        (:`3`
          (`/Game/KIA_Game/template/template_BP/BP_KartPawnBase.UseTeleport` _aipawnref))))))

(fn `UserConstructionScript`)