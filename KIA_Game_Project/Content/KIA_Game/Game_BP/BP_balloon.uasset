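; BP_balloon is a hot air balloon actor that takes on a random color and moves with a timeline-driven bounce.
; On BeginPlay it picks one of four striped balloon meshes at random and records its spawn location.
; A timeline then lerps the actor between that location and an offset set by BounceZonly, without sweeping for collision.
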(event `self.ReceiveBeginPlay`
  (bind _spawn_location (`self.spawn location`))
  (`StaticMeshComponent.SetStaticMesh` (`self.StaticMesh`) (`KismetArrayLibrary.Array_Random` (`|MakeArray` "/Game/KIA_Game/Assets_KIA/Meshes/Scenery/Hotair_Balloon/Hotair_Balloon_CyanandGreen_Mesh.Hotair_Balloon_CyanandGreen_Mesh" "/Game/KIA_Game/Assets_KIA/Meshes/Scenery/Hotair_Balloon/Hotair_Balloon_RedandWhite_Mesh.Hotair_Balloon_RedandWhite_Mesh" "/Game/KIA_Game/Assets_KIA/Meshes/Scenery/Hotair_Balloon/Hotair_Balloon_YellowandBlue_Mesh.Hotair_Balloon_YellowandBlue_Mesh" "/Game/KIA_Game/Assets_KIA/Meshes/Scenery/Hotair_Balloon/Hotair_Balloon_YellowandOrange_Mesh.Hotair_Balloon_YellowandOrange_Mesh" :!type "StaticMesh Object Reference")))
  (set `self.spawn location` (`self.K2_GetActorLocation`))
  (bind (_direction _newtrack_0) (`Timeline|Timeline_0`)
    (:`Update`
      (`self.K2_SetActorLocation` (`KismetMathLibrary.VLerp` _spawn_location (+ _spawn_location (`self.bounce(Zonly)`)) _newtrack_0)))))

(fn `UserConstructionScript`)