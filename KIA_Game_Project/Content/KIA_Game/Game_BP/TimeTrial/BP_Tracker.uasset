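; Time trial race tracker that runs a kart course's ordered checkpoints and passes lap count, save name, map and medal times to the player controller.
; It numbers and binds checkpoints, then on each clear authorizes the kart on the next one and records respawn points.
; Player and AI karts use parallel lap and completion checks; only the player path unhides checkpoints.
; Completion triggers the end-race camera; AI laps update only when already complete.
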(event `self.ReceiveBeginPlay`
  ;[1 1 1] Game init
  (bind _asbp_player_controller (cast `/Game/KIA_Game/Game_BP/TimeTrial/BP_PlayerController` (`GameplayStatics.GetPlayerController` 0)))
  (set `self.As BP Player Controller` _asbp_player_controller)
  (`self.applySettings`)
  (`self.StartSequance`))

(event `applySettings`
  (bind _as_bp_player_controller (`self.As BP Player Controller`))
  ;[1 1 1] Apply user settings when starting
  (set `/Game/KIA_Game/Game_BP/TimeTrial/BP_PlayerController.MaxLap` (`self.MaxLap`) _as_bp_player_controller)
  (set `/Game/KIA_Game/Game_BP/TimeTrial/BP_PlayerController.Save` (`self.SaveGameName`) _as_bp_player_controller)
  (set `/Game/KIA_Game/Game_BP/TimeTrial/BP_PlayerController.NameOfMap` (`self.NameOfMap`) _as_bp_player_controller)
  (`self.UpdateTime`)
  (`/Game/KIA_Game/Game_BP/TimeTrial/BP_PlayerController.StartGAme` _as_bp_player_controller)
  (`self.StartSequance`))

(event `StartSequance`
  (bind _checkpoints (`self.CheckPoints`))
  ;[1 1 1] Activate and clear all checkpoints
  (for (_array_element _array_index) (`self.CheckPoints`)
    (set `/Game/KIA_Game/Game_BP/TimeTrial/BP_CheckPoint.CheckPointNumber` (+ _array_index 1) _array_element)
    (set `self.TotalCheckPoints` (`KismetArrayLibrary.Array_Length` _checkpoints))
    (`self.ActivateCheckpoint` (`|GetArrayItem` _checkpoints))
    (for _array_element_2 (`self.CheckPoints`)
      (add `/Game/KIA_Game/Game_BP/TimeTrial/BP_CheckPoint.CheckPointCleared` _array_element_2 (delegate `CheckPointCleared`)))))

(event `CheckPointCleared`
  (params (NextCheckPoint :type Integer) (Kart :type "Pawn Object Reference") (Player :type Boolean))
  (bind _as_bp_player_controller (`self.As BP Player Controller`))
  ;[1 1 1] CheckAllCheckpointCleared
  (if Player
    (`self.LapCheck` NextCheckPoint Kart)
    (`GameplayStatics.PlaySoundAtLocation` (`self.SoundFx`) (0.0 0.0 0.0) (struct) 1.0 1.0 0.0 null null null)
    (if (`/Game/KIA_Game/Game_BP/TimeTrial/BP_PlayerController.RaceComplete` _as_bp_player_controller)
      (`/Game/KIA_Game/Game_BP/TimeTrial/BP_PlayerController.SetToEndRaceCamera` _as_bp_player_controller))
    (else
      (bind _asbp_aicontroller (cast `/Game/KIA_Game/template/template_BP/BasicAI/BP_AIController` (`AIBlueprintHelperLibrary.GetAIController` Kart)))
      (set `self.As BP AIController` _asbp_aicontroller)
      (`self.LapCheckAI` NextCheckPoint Kart)
      (`KismetSystemLibrary.PrintString` "After lap check AI")
      (if (`/Game/KIA_Game/template/template_BP/BasicAI/BP_AIController.RaceComplete` (`self.As BP AIController`))
        (`/Game/KIA_Game/Game_BP/TimeTrial/BP_PlayerController.SetToEndRaceCamera` _as_bp_player_controller)))))

(fn `ActivateCheckpoint`
  (params (CheckPoint :type "/Game/KIA_Game/Game_BP/TimeTrial/BP_CheckPoint Object Reference") (Kart :type "Pawn Object Reference"))
  (bind _dection (`/Game/KIA_Game/Game_BP/TimeTrial/BP_CheckPoint.Dection` CheckPoint))
  ;[1 1 1] ActivateNextCheckpoint
  (`KismetArrayLibrary.Array_Add` (`/Game/KIA_Game/Game_BP/TimeTrial/BP_CheckPoint.AuthorizedKart` CheckPoint) Kart)
  (`SceneComponent.SetHiddenInGame` _dection false false)
  (set `PrimitiveComponent.bGenerateOverlapEvents` true _dection))

(fn `ActivateCheckpointAI`
  (params (CheckPoint :type "/Game/KIA_Game/Game_BP/TimeTrial/BP_CheckPoint Object Reference") (Kart :type "Pawn Object Reference"))
  ;[1 1 1] ActivateNextCheckpoint
  (`KismetSystemLibrary.PrintString` "In activate checkpoint AI")
  (`KismetArrayLibrary.Array_Add` (`/Game/KIA_Game/Game_BP/TimeTrial/BP_CheckPoint.AuthorizedKart` CheckPoint) Kart)
  (set `PrimitiveComponent.bGenerateOverlapEvents` true (`/Game/KIA_Game/Game_BP/TimeTrial/BP_CheckPoint.Dection` CheckPoint)))

(fn `LapCheck`
  (params (Checkpoint :type Integer) (Kart :type "Pawn Object Reference"))
  (locals (LocalCheckPoint :type Integer))
  ;[1 1 1] CheckCheckpoint_Lap_RaceComplete
  (bind _output_get (set `local.LocalCheckPoint` Checkpoint))
  (if (== _output_get (`self.TotalCheckPoints`))
    (bind _israce_over (`self.RaceCompleteCheck`))
    (if (not _israce_over)
      (`self.ActivateCheckpoint` (`|GetArrayItem` (`self.CheckPoints`)) Kart))
    (`/Game/KIA_Game/Game_BP/TimeTrial/BP_PlayerController.UpdateLap` (`self.As BP Player Controller`))
    (else
      (`self.ActivateCheckpoint` (`|GetArrayItem` (`self.CheckPoints`) (`local.LocalCheckPoint`)) Kart)))
  (set `/Game/KIA_Game/Game_BP/TimeTrial/BP_PlayerController.RespawnLoco` (`self.GetTransform` (`|GetArrayItem` (`self.CheckPoints`) (- (`local.LocalCheckPoint`) 1))) (`self.As BP Player Controller`)))

(fn `LapCheckAI`
  (params (Checkpoint :type Integer) (Kart :type "Pawn Object Reference"))
  (locals (LocalCheckPoint :type Integer))
  ;[1 1 1] CheckCheckpoint_Lap_RaceComplete
  (`KismetSystemLibrary.PrintString` "Inside LapCheckAI")
  (bind _output_get (set `local.LocalCheckPoint` Checkpoint))
  (if (== _output_get (`self.TotalCheckPoints`))
    (bind _israce_over (`self.RaceCompleteCheckAI`))
    (if _israce_over
      (`/Game/KIA_Game/template/template_BP/BasicAI/BP_AIController.UpdateLap` (`self.As BP AIController`))
      (set `/Game/KIA_Game/template/template_BP/BasicAI/BP_AIController.RespawnLocation` (`self.GetTransform` (`|GetArrayItem` (`self.CheckPoints`) (- (`local.LocalCheckPoint`) 1))) (`self.As BP AIController`) :!label _label)
      (else
        (`self.ActivateCheckpointAI` (`|GetArrayItem` (`self.CheckPoints`)) Kart)))
    (else
      (`self.ActivateCheckpointAI` (`|GetArrayItem` (`self.CheckPoints`) (`local.LocalCheckPoint`)) Kart)
      (goto _label))))

(fn `RaceCompleteCheck`
  (returns (`isRAce over` :type Boolean))
  (locals (LocalComplete :type Boolean))
  (bind _as_bp_player_controller (`self.As BP Player Controller`))
  ;[1 1 1] CheckAndSetRaceComplete
  (if (>= (`/Game/KIA_Game/Game_BP/TimeTrial/BP_PlayerController.ActualLap` _as_bp_player_controller) (`/Game/KIA_Game/Game_BP/TimeTrial/BP_PlayerController.MaxLap` _as_bp_player_controller))
    (bind _output_get (set `/Game/KIA_Game/Game_BP/TimeTrial/BP_PlayerController.RaceComplete` true _as_bp_player_controller))
    (set `local.LocalComplete` _output_get)
    (else
      (bind _output_get_2 (set `/Game/KIA_Game/Game_BP/TimeTrial/BP_PlayerController.RaceComplete` false _as_bp_player_controller))
      (set `local.LocalComplete` _output_get_2)))
  (return (`local.LocalComplete`)))

(fn `RaceCompleteCheckAI`
  (returns (`isRAce over` :type Boolean))
  (locals (LocalComplete :type Boolean))
  (bind _as_bp_aicontroller (`self.As BP AIController`))
  ;[1 1 1] CheckAndSetRaceComplete
  (`KismetSystemLibrary.PrintString` "Entered Race complete check AI")
  (if (>= (`/Game/KIA_Game/template/template_BP/BasicAI/BP_AIController.ActualLap` _as_bp_aicontroller) (`/Game/KIA_Game/template/template_BP/BasicAI/BP_AIController.MaxLap` _as_bp_aicontroller))
    (bind _output_get (set `/Game/KIA_Game/template/template_BP/BasicAI/BP_AIController.RaceComplete` true _as_bp_aicontroller))
    (set `local.LocalComplete` _output_get)
    (else
      (bind _output_get_2 (set `/Game/KIA_Game/template/template_BP/BasicAI/BP_AIController.RaceComplete` false _as_bp_aicontroller))
      (set `local.LocalComplete` _output_get_2)))
  (return (`local.LocalComplete`)))

(fn `UpdateTime`
  (bind _as_bp_player_controller (`self.As BP Player Controller`))
  ;[1 1 1] PassUserTimesToPlayerControllerTimes
  (set `/Game/KIA_Game/Game_BP/TimeTrial/BP_PlayerController.GoldTime` (`self.GoldTime`) _as_bp_player_controller)
  (set `/Game/KIA_Game/Game_BP/TimeTrial/BP_PlayerController.SilverTime` (`self.Silver`) _as_bp_player_controller)
  (set `/Game/KIA_Game/Game_BP/TimeTrial/BP_PlayerController.BronzeTime` (`self.Bronze`) _as_bp_player_controller)
  (set `/Game/KIA_Game/Game_BP/TimeTrial/BP_PlayerController.BestRaceTime` (`self.Defult BestRace`) _as_bp_player_controller)
  (set `/Game/KIA_Game/Game_BP/TimeTrial/BP_PlayerController.BestLapTime` (`self.Defult BestLap`) _as_bp_player_controller))

(fn `UpdateTimeAI`
  (bind _as_bp_player_controller (`self.As BP Player Controller`))
  ;[1 0.1335 0.9721] PassUserTimesToPlayerControllerTimes NOTUPDATEORUSEDBYAIYET
  (set `/Game/KIA_Game/Game_BP/TimeTrial/BP_PlayerController.GoldTime` (`self.GoldTime`) _as_bp_player_controller)
  (set `/Game/KIA_Game/Game_BP/TimeTrial/BP_PlayerController.SilverTime` (`self.Silver`) _as_bp_player_controller)
  (set `/Game/KIA_Game/Game_BP/TimeTrial/BP_PlayerController.BronzeTime` (`self.Bronze`) _as_bp_player_controller)
  (set `/Game/KIA_Game/Game_BP/TimeTrial/BP_PlayerController.BestRaceTime` (`self.Defult BestRace`) _as_bp_player_controller)
  (set `/Game/KIA_Game/Game_BP/TimeTrial/BP_PlayerController.BestLapTime` (`self.Defult BestLap`) _as_bp_player_controller))

(fn `UserConstructionScript`)