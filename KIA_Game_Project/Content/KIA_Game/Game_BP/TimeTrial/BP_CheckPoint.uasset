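; Time trial checkpoint actor that registers when a player kart passes through it in the correct direction.
; When a kart pawn leaves the detection component, a dot product of its velocity and the Arrow's forward vector rejects wrong-way crossings.
; A valid pass broadcasts CheckPointCleared with the checkpoint number, then hides the detection component and disables its overlaps so it fires only once.
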(event `self.Dection.OnComponentEndOverlap`
  (params (OverlappedComponent :type "PrimitiveComponent Object Reference") (OtherActor :type "Actor Object Reference") (OtherComp :type "PrimitiveComponent Object Reference") (OtherBodyIndex :type Integer))
  (bind _dection (`self.Dection`))
  ;[1 1 1] ChecKpoint Clearer
  (bind _asbp_kart_pawn_base_child (cast `/Game/KIA_Game/template/template_BP/BP_KartPawnBase_Child` OtherActor))
  (if (> (`KismetMathLibrary.Dot_VectorVector` (`self.GetVelocity` _asbp_kart_pawn_base_child) (`KismetMathLibrary.Conv_RotatorToVector` (`SceneComponent.K2_GetComponentRotation` (`self.Arrow`)))) 0.0)
    (`self.CheckPointCleared` (`self.CheckPointNumber`))
    (`SceneComponent.SetHiddenInGame` _dection true false)
    (set `PrimitiveComponent.bGenerateOverlapEvents` false _dection)))

(fn `UserConstructionScript`)