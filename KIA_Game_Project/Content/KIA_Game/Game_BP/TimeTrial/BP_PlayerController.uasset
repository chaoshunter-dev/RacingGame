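; Player controller for the kart time trial, running the countdown, lap and race timing, HUD text and best-time records.
; A one-shot left click starts the countdown, then two Timelines act as race and lap stopwatches, with race updates hiding missed gold, silver and bronze goals.
; UpdateLap compares times against bests, saving records to BP_savegame and playing HUD animations.
; It also handles respawn, level restart and a pre-race R-key record reset.
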(event `self.ReceiveBeginPlay`
  ;[1 1 1] GetReference
  (bind _returnvalue (`|CreateWidget` "/Game/KIA_Game/Game_BP/TimeTrial/WID_HUD.WID_HUD_C"))
  (bind _output_get (set `self.HUDReference` _returnvalue))
  (`UserWidget.AddToViewport` _output_get 0)
  (bind _asbp_kart_pawn_base_child (cast `/Game/KIA_Game/template/template_BP/BP_KartPawnBase_Child` (`GameplayStatics.GetPlayerPawn` 0)))
  (set `self.PAWNRef` _asbp_kart_pawn_base_child))

(event `StartRace time`
  ;[1 1 1] RaceAndLapsTimersToText
  (bind (_direction _time) (`Timeline|Timeline_0` :!label _label)
    (:`Update`
      (bind _output_get (set `self.Racetime` _time))
      (set `self.RaceTimeText` (`/Game/KIA_Game/Game_BP/TimeTrial/BP_TimeConvertor.TimetoText` _output_get))
      (`self.UpdateGoal`))))

(event `StopRaceTimes`
  ;[1 1 1] RaceAndLapsTimersToText
  (goto _label :!via `Stop`))

(event `StartLaptime`
  ;[1 1 1] RaceAndLapsTimersToText
  (bind (_direction _time) (`Timeline|Timeline_1` :!via `PlayFromStart` :!label _label_2)
    (:`Update`
      (set `self.LapTime` _time))))

(event `StartGame`
  ;[1 1 1] StartAndCheckForSave
  (`self.SaveGameCheck`)
  (`self.InitText`))

(event `stopLapTime`
  ;[1 1 1] RaceAndLapsTimersToText
  (goto _label_2 :!via `Stop`))

(event `Restart`
  ;[1 1 1] RestartWhenRaceComplete
  (set `self.RaceStart` false)
  (`KismetSystemLibrary.Delay` 6.0)
  (`KismetSystemLibrary.ExecuteConsoleCommand` "RestartLevel" null))

(event `Key|R`
  (params (Key :type "Key Structure"))
  ;[1 1 1] ResetDefaultBestTime
  (:`Pressed`
    (if (not (`self.RaceStart`))
      (set `self.BestLapTime` (`self.DefaultLapTime_1`))
      (set `self.BestRaceTime` (`self.DefaultRaceTime_0`))
      (`self.SaveGame`)
      (`self.InitText`))))

(event `UpdateLap`
  ;[1 1 1] updateLaps
  (if (not (`self.RaceComplete`))
    (bind _output_get (set `self.ActualLap` (+ (`self.ActualLap`) 1)))
    (set `self.CurrentLapText` (`KismetTextLibrary.Conv_IntToText` _output_get)))
  (`self.LapTimeCheck`))

(event `Respawn`
  (bind (_respawnloco_location _respawnloco_rotation) (`KismetMathLibrary.BreakTransform` (`self.RespawnLoco`)))
  ;[1 1 1] Plug scale in for a goood time
  (bind _returnvalue (`|SpawnActorFromClass` "/Game/KIA_Game/Assets_KIA/Blueprints/Trainkart_BP.Trainkart_BP_C" (`KismetMathLibrary.MakeTransform` _respawnloco_location _respawnloco_rotation) "Undefined" "OverrideRootScale" null null))
  (`self.Possess` _returnvalue))

(event `Key|LeftMouseButton`
  (params (Key :type "Key Structure"))
  (bind _hudreference (`self.HUDReference`))
  ;[1 1 1] LeftClickToStartAndSetHUDsVisibility
  (:`Pressed`
    (`/Engine/EditorBlueprintResources/StandardMacros.DoOnce` false
      (:`Completed`
        (set `/Game/KIA_Game/Game_BP/TimeTrial/WID_HUD.SplashScreenVisible` "Hidden" _hudreference)
        (set `/Game/KIA_Game/Game_BP/TimeTrial/WID_HUD.CountDownVisible` "Visible" _hudreference)
        (`KismetSystemLibrary.Delay` 1.0)
        (`GameplayStatics.PlaySoundAtLocation` "/Game/KIA_Game/audio/get_set.get_set" (0.0 0.0 0.0) (struct) 1.0 1.0 0.0 null null null)
        (`self.lightstart`)
        (set `self.ReadyText` "2")
        (`KismetSystemLibrary.Delay` 1.0)
        (set `self.ReadyText` "1")
        (`KismetSystemLibrary.Delay` 1.0)
        (set `self.ReadyText` "GO!")
        (set `/Game/KIA_Game/Game_BP/TimeTrial/WID_HUD.GameHUDVisible` "Visible" (`self.HUDReference`))
        (set `self.RaceStart` true)
        (`self.StartRace time`)
        (`self.StartLaptime`)
        (`KismetSystemLibrary.Delay` 0.6)
        (set `/Game/KIA_Game/Game_BP/TimeTrial/WID_HUD.CountDownVisible` "Hidden" (`self.HUDReference`))))))

(event `SetToEndRaceCamera`
  (`/Game/KIA_Game/template/template_BP/BP_KartPawnBase.EndRaceCamera` (`self.PAWNRef`)))

(event `Key|U`
  (params (Key :type "Key Structure"))
  ;[1 1 1] DebugOnly DisplayTimer
  (:`Pressed`
    (set `self.ReadyText` (`/Game/KIA_Game/Game_BP/TimeTrial/BP_TimeConvertor.TimetoText` (`self.BestLapTime`)))
    (set `self.RaceTimeText` (`/Game/KIA_Game/Game_BP/TimeTrial/BP_TimeConvertor.TimetoText` (`self.BestRaceTime`)))
    (`KismetSystemLibrary.PrintText` (`self.ReadyText`))
    (`KismetSystemLibrary.PrintText` (`self.RaceTimeText`))))

(event `self.ReceiveTick`
  (params (DeltaSeconds :type "Float (single-precision)")))

(fn `InitText`
  ;[1 1 1] ConvertAllTimesToText
  (set `self.CurrentLapText` (`KismetTextLibrary.Conv_IntToText` (`self.ActualLap`)))
  (set `self.MaxLapText` (`KismetTextLibrary.Conv_IntToText` (`self.MaxLap`)))
  (set `self.GoldText` (`/Game/KIA_Game/Game_BP/TimeTrial/BP_TimeConvertor.TimetoText` (`self.GoldTime`)))
  (set `self.SilverText` (`/Game/KIA_Game/Game_BP/TimeTrial/BP_TimeConvertor.TimetoText` (`self.SilverTime`)))
  (set `self.BronzeText` (`/Game/KIA_Game/Game_BP/TimeTrial/BP_TimeConvertor.TimetoText` (`self.BronzeTime`)))
  (set `self.BestLapText` (`/Game/KIA_Game/Game_BP/TimeTrial/BP_TimeConvertor.TimetoText` (`self.BestLapTime`)))
  (set `self.BestTimeText` (`/Game/KIA_Game/Game_BP/TimeTrial/BP_TimeConvertor.TimetoText` (`self.BestRaceTime`))))

(fn `LapTimeCheck`
  (bind _bestlaptime (`self.BestLapTime`))
  (bind _hudreference (`self.HUDReference`))
  ;[1 1 1] LapTimeCheckAndSaveBestLap
  (`self.stopLapTime`)
  (if (<= (`self.LapTime`) _bestlaptime)
    (bind _output_get (set `self.BestLapTime` (`self.LapTime`)))
    (set `self.BestLapText` (`/Game/KIA_Game/Game_BP/TimeTrial/BP_TimeConvertor.TimetoText` _output_get))
    (`self.SaveGame`)
    (`UserWidget.PlayAnimation` _hudreference (`/Game/KIA_Game/Game_BP/TimeTrial/WID_HUD.LapAnimation` _hudreference) 0.0 1 "Forward" 1.0 false)
    (set `self.LapTime` 0.0)
    (else
      (`KismetSystemLibrary.PrintString` "Pa  de meileur temps laps")
      (`KismetSystemLibrary.PrintString` (`KismetStringLibrary.Conv_DoubleToString` _bestlaptime))
      (set `self.LapTime` 0.0)))
  (if (`self.RaceComplete`)
    (`self.RaceTimeCheck`)
    (else
      (`self.StartLAptime`))))

(fn `LoadGame`
  (bind _returnvalue (`GameplayStatics.LoadGameFromSlot` (`self.Save`)))
  (bind _asbp_savegame (cast `/Game/KIA_Game/Game_BP/TimeTrial/BP_savegame` _returnvalue))
  (set `self.BestRaceTime` (`/Game/KIA_Game/Game_BP/TimeTrial/BP_savegame.SaveBestRace` _asbp_savegame))
  (set `self.BestLapTime` (`/Game/KIA_Game/Game_BP/TimeTrial/BP_savegame.SaveBestLap` _asbp_savegame)))

(fn `RaceTimeCheck`
  (bind _hudreference (`self.HUDReference`))
  ;[1 1 1] RaceTimeCheckAndSaveBestRace
  (`self.StopRaceTimes`)
  (if (<= (`self.Racetime`) (`self.BestRaceTime`))
    (bind _output_get (set `self.BestRaceTime` (`self.Racetime`)))
    (set `self.BestTimeText` (`/Game/KIA_Game/Game_BP/TimeTrial/BP_TimeConvertor.TimetoText` _output_get))
    (`self.SaveGame`)
    (`UserWidget.PlayAnimation` _hudreference (`/Game/KIA_Game/Game_BP/TimeTrial/WID_HUD.RaceRecordAnimation` _hudreference) 0.0 1 "Forward" 1.0 false)))

(fn `SaveGame`
  (bind _returnvalue (`GameplayStatics.CreateSaveGameObject` "/Game/KIA_Game/Game_BP/TimeTrial/BP_savegame.BP_savegame_C"))
  (bind _output_get (set `self.savefile` _returnvalue))
  (set `/Game/KIA_Game/Game_BP/TimeTrial/BP_savegame.SaveBestLap` (`self.BestLapTime`) _output_get)
  (set `/Game/KIA_Game/Game_BP/TimeTrial/BP_savegame.SaveBestRace` (`self.BestRaceTime`) _output_get)
  (`GameplayStatics.SaveGameToSlot` (`self.savefile`) (`self.Save`)))

(fn `SaveGameCheck`
  ;[1 1 1] CheckForSavedGameAndLoadOrLoadDefault
  (bind _returnvalue (`GameplayStatics.DoesSaveGameExist` (`self.Save`)))
  (if _returnvalue
    (`self.LoadGame`)
    (else
      (set `self.BestRaceTime` (`self.DefaultRaceTime_0`))
      (set `self.BestLapTime` (`self.DefaultLapTime_1`))
      (`self.SaveGame`))))

(fn `UpdateGoal`
  ;[1 1 1] SetGold/Silver/BronzeToHidden
  (if (not (<= (`self.Racetime`) (`self.GoldTime`)))
    (`|ExecutionSequence`
      (:`then_0`
        (`/Engine/EditorBlueprintResources/StandardMacros.DoOnce` false
          (:`Completed`
            (set `/Game/KIA_Game/Game_BP/TimeTrial/WID_HUD.GoldTimeVisible` "Hidden" (`self.HUDReference`)))))
      (:`then_1`
        (if (not (<= (`self.Racetime`) (`self.SilverTime`)))
          (`|ExecutionSequence`
            (:`then_0`
              (`/Engine/EditorBlueprintResources/StandardMacros.DoOnce` false
                (:`Completed`
                  (set `/Game/KIA_Game/Game_BP/TimeTrial/WID_HUD.SilverTimeVisible` "Hidden" (`self.HUDReference`)))))
            (:`then_1`
              (if (not (<= (`self.Racetime`) (`self.BronzeTime`)))
                (`/Engine/EditorBlueprintResources/StandardMacros.DoOnce` false
                  (:`Completed`
                    (set `/Game/KIA_Game/Game_BP/TimeTrial/WID_HUD.BronzeTimeVisible` "Hidden" (`self.HUDReference`))))))))))))

(fn `UserConstructionScript`)