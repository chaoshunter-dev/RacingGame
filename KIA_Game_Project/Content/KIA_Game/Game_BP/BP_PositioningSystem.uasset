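; Race positioning actor that ranks all karts and writes each one's place to its AI or player controller.
; BeginPlay caches karts and controllers, then enables an interval-throttled Tick that runs until the player's race completes.
; Each pass, gated by a DoOnce, rebuilds a struct array of lap and spline distance per kart.
; A bubble sort orders it descending, swapping when either lap or distance is lower, so distance can override lap.
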(event `self.ReceiveBeginPlay`
  (bind _controllersrefs (`self.ControllersRefs`))
  ;[1 1 1] PositioningSystem
  (`self.SetActorTickEnabled` false)
  (bind _asbp_player_controller (cast `/Game/KIA_Game/Game_BP/TimeTrial/BP_PlayerController` (`GameplayStatics.GetPlayerController` 0)))
  (set `self.PlayerControllerRef` _asbp_player_controller)
  (bind _outactors (`GameplayStatics.GetAllActorsOfClass` "/Game/KIA_Game/template/template_BP/BP_KartPawnBase.BP_KartPawnBase_C"))
  (bind _output_get (set `self.KartsRefs` _outactors))
  (for _array_element _output_get
    (bind _asbp_kart_pawn_base_ai_temp (cast `/Game/KIA_Game/template/template_BP/BasicAI/BP_KartPawnBase_AiTemp` _array_element)
      (:`then`
        (`KismetArrayLibrary.Array_Add` _controllersrefs (`Pawn.GetController` _asbp_kart_pawn_base_ai_temp)))
      (:`CastFailed`
        (bind _astest_improvement_of_ai (cast `/Game/KIA_Game/template/template_BP/BasicAI/TestImprovementOfAI` _array_element)
          (:`then`
            (`KismetArrayLibrary.Array_Add` _controllersrefs (`Pawn.GetController` _astest_improvement_of_ai)))
          (:`CastFailed`
            (`KismetArrayLibrary.Array_Add` _controllersrefs (`GameplayStatics.GetPlayerController` 0)))))))
  (`self.SetActorTickInterval` 0.5)
  (`self.SetActorTickEnabled` true))

(event `self.ReceiveTick`
  (params (DeltaSeconds :type "Float (single-precision)"))
  ;[1 1 1] PositioningSystem
  (if (not (`/Game/KIA_Game/Game_BP/TimeTrial/BP_PlayerController.RaceComplete` (`self.PlayerControllerRef`)))
    (`/Engine/EditorBlueprintResources/StandardMacros.DoOnce` false :!label _label
      (:`Completed`
        (for _array_element (`self.KartsRefs`)
          (`/Game/KIA_Game/template/template_BP/BP_KartPawnBase.Get Spline Point Distance` _array_element)
          (`self.UpdateStructArray` _array_element (`/Game/KIA_Game/template/template_BP/BP_KartPawnBase.DistanceToSpline` _array_element)))
        (bind _kartanddistance (`self.SortAlgorithm` (`self.KartAndDistance`)))
        (for (_array_element_2 _array_index) _kartanddistance
          (set `self.TempArrayIndex` (+ _array_index 1))
          (bind (_kartrefs _controllerref) (break `/Game/KIA_Game/Game_BP/TimeTrial/PositioningStruct` _array_element_2))
          (set `self.TempKartRef` _kartrefs)
          (set `self.TempControllerRef` _controllerref)
          (bind _asbp_aicontroller (cast `/Game/KIA_Game/template/template_BP/BasicAI/BP_AIController` (`self.TempControllerRef`))
            (:`then`
              (bind _output_get (set `/Game/KIA_Game/template/template_BP/BasicAI/BP_AIController.Position` (`self.TempArrayIndex`) _asbp_aicontroller)))
            (:`CastFailed`
              (bind _asbp_player_controller (cast `/Game/KIA_Game/Game_BP/TimeTrial/BP_PlayerController` (`self.TempControllerRef`)))
              (bind _output_get_2 (set `/Game/KIA_Game/Game_BP/TimeTrial/BP_PlayerController.Position` (`self.TempArrayIndex`) _asbp_player_controller)))))
        (`KismetSystemLibrary.Delay` 0.2)
        (`KismetArrayLibrary.Array_Clear` (`self.KartAndDistance`))
        (set `self.IndexControllerRef` 0)
        (`self.LoopCompleted`)))))

(event `LoopCompleted`
  ;[1 1 1] PositioningSystem
  (goto _label :!via `Reset`))

(fn `SortAlgorithm`
  (params (ArrayToSort :type "Array of /Game/KIA_Game/Game_BP/TimeTrial/PositioningStruct Structure"))
  (returns (KartAndDistance :type "Array of /Game/KIA_Game/Game_BP/TimeTrial/PositioningStruct Structure"))
  (bind _returnvalue (- (`KismetArrayLibrary.Array_Length` ArrayToSort) 1))
  (for _index (range (+ _returnvalue 1))
    (for _index_2 (range (- _returnvalue _index))
      (bind (_kartrefs _controllerref _distanceonspline _actuallap) (break `/Game/KIA_Game/Game_BP/TimeTrial/PositioningStruct` (`|GetArrayItem` ArrayToSort _index_2)))
      (bind _returnvalue_2 (+ _index_2 1))
      (bind (_kartrefs_2 _controllerref_2 _distanceonspline_2 _actuallap_2) (break `/Game/KIA_Game/Game_BP/TimeTrial/PositioningStruct` (`|GetArrayItem` ArrayToSort _returnvalue_2)))
      (if (< _actuallap _actuallap_2)
        (`KismetArrayLibrary.Array_Swap` ArrayToSort _index_2 _returnvalue_2 :!label _label)
        (elif (< _distanceonspline _distanceonspline_2)
          (goto _label)))))
  (return (`self.KartAndDistance`)))

(fn `UpdateStructArray`
  (params (KartRef :type "/Game/KIA_Game/template/template_BP/BP_KartPawnBase Object Reference") (DistanceOnSpline :type "Float (double-precision)"))
  (locals (TempActualLap :type Integer))
  (bind _output (`|GetArrayItem` (`self.ControllersRefs`) (`self.IndexControllerRef`)))
  (bind _asbp_aicontroller (cast `/Game/KIA_Game/template/template_BP/BasicAI/BP_AIController` _output)
    (:`then`
      (set `local.TempActualLap` (`/Game/KIA_Game/template/template_BP/BasicAI/BP_AIController.ActualLap` _asbp_aicontroller)))
    (:`CastFailed`
      (bind _asbp_player_controller (cast `/Game/KIA_Game/Game_BP/TimeTrial/BP_PlayerController` _output))
      (set `local.TempActualLap` (`/Game/KIA_Game/Game_BP/TimeTrial/BP_PlayerController.ActualLap` _asbp_player_controller))))
  (`KismetArrayLibrary.Array_Add` (`self.KartAndDistance`) (make `/Game/KIA_Game/Game_BP/TimeTrial/PositioningStruct` KartRef _output DistanceOnSpline (`local.TempActualLap`)))
  (`/Engine/EditorBlueprintResources/StandardMacros.IncrementInt` (`self.IndexControllerRef`)))

(fn `UserConstructionScript`)