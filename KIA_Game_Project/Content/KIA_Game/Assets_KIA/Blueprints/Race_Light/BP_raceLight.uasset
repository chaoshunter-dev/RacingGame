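; BP_raceLight is the race start light that runs the countdown and releases the player's kart.
; On BeginPlay it binds its LightsSwitch event to the light-start dispatcher on BP_PlayerController.
; The sequence lights red, amber and green through material scalar parameters one second apart, each with a sound.
; It then enables input on the player's BP_KartPawnBase_Child and switches all lights off a few seconds later.
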(event `self.ReceiveBeginPlay`
  (bind _returnvalue (`GameplayStatics.GetActorOfClass` "/Game/KIA_Game/Game_BP/TimeTrial/BP_PlayerController.BP_PlayerController_C"))
  (add `/Game/KIA_Game/Game_BP/TimeTrial/BP_PlayerController.lightstart` _returnvalue (delegate `lights switch`)))

(event `lights switch`
  (bind _staticmesh (`self.StaticMesh`))
  (bind _asbp_kart_pawn_base_child (cast `/Game/KIA_Game/template/template_BP/BP_KartPawnBase_Child` (`GameplayStatics.GetPlayerPawn` 0)))
  (`KismetSystemLibrary.Delay` 0.0)
  (`MeshComponent.SetScalarParameterValueOnMaterials` _staticmesh "redlight" 1.0)
  (`GameplayStatics.PlaySoundAtLocation` null (0.0 0.0 0.0) (struct) 1.0 1.0 0.0 null null null)
  (`KismetSystemLibrary.Delay` 1.0)
  (`MeshComponent.SetScalarParameterValueOnMaterials` _staticmesh "AmberLight" 1.0)
  (`GameplayStatics.PlaySoundAtLocation` "/Game/KIA_Game/audio/get_set.get_set" (0.0 0.0 0.0) (struct) 1.0 1.0 0.0 null null null)
  (`KismetSystemLibrary.Delay` 1.0)
  (`MeshComponent.SetScalarParameterValueOnMaterials` _staticmesh "greenLight" 1.0)
  (`GameplayStatics.PlaySoundAtLocation` "/Game/KIA_Game/audio/lap_completion.lap_completion" (0.0 0.0 0.0) (struct) 1.0 1.0 0.0 null null null)
  (`KismetSystemLibrary.Delay` 1.0)
  (`self.EnableInput` _asbp_kart_pawn_base_child null)
  (`KismetSystemLibrary.Delay` 5.0)
  (`MeshComponent.SetScalarParameterValueOnMaterials` _staticmesh "redlight" 0.0)
  (`MeshComponent.SetScalarParameterValueOnMaterials` _staticmesh "AmberLight" 0.0)
  (`MeshComponent.SetScalarParameterValueOnMaterials` _staticmesh "greenLight" 0.0))

(fn `UserConstructionScript`)