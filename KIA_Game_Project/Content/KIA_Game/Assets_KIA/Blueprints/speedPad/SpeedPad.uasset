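; SpeedPad is a boost pad that launches karts that overlap its Box trigger.
; It adds velocity along the Arrow's forward vector, scaled by BlastSpeed, to the kart's collision component.
; A DoOnce gate blocks retriggering until BoostCooldown elapses, so one cooldown is shared by all karts.
; The Plane turns red during cooldown and green afterwards, using a newly created dynamic material instance each time.
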(event `self.Box.OnComponentBeginOverlap`
  (params (OverlappedComponent :type "PrimitiveComponent Object Reference") (OtherActor :type "Actor Object Reference") (OtherComp :type "PrimitiveComponent Object Reference") (OtherBodyIndex :type Integer) (bFromSweep :type Boolean) (SweepResult :type "HitResult Structure (by ref)"))
  (bind _plane (`self.Plane`))
  (bind _asbp_kart_pawn_base (cast `/Game/KIA_Game/template/template_BP/BP_KartPawnBase` OtherActor))
  (`/Engine/EditorBlueprintResources/StandardMacros.DoOnce` false :!label _label
    (:`Completed`
      (bind _returnvalue (`PrimitiveComponent.CreateDynamicMaterialInstance` _plane 0 "/Game/KIA_Game/Assets_KIA/Materials/Scenery/boostpad/arrow.arrow" "None"))
      (`MaterialInstanceDynamic.SetVectorParameterValue` _returnvalue "colour" (struct :`R` 0.947917 :`G` 0.113647 :`A` 1.0))
      (`PrimitiveComponent.SetPhysicsLinearVelocity` (`/Game/KIA_Game/template/template_BP/BP_KartPawnBase.Kart_Collision` _asbp_kart_pawn_base) (* (`SceneComponent.GetForwardVector` (`self.Arrow`)) (`self.blastSpeed`)) true "None")
      (`KismetSystemLibrary.Delay` (`self.boost cooldown`))
      (bind _returnvalue_2 (`PrimitiveComponent.CreateDynamicMaterialInstance` _plane 0 "/Game/KIA_Game/Assets_KIA/Materials/Scenery/boostpad/arrow.arrow" "None"))
      (`MaterialInstanceDynamic.SetVectorParameterValue` _returnvalue_2 "colour" (struct :`R` 0.005605 :`G` 0.597202 :`B` 0.000911 :`A` 1.0))
      (goto _label :!via `Reset`))))

(fn `UserConstructionScript`)