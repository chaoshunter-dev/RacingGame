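; Player-driven wheeled vehicle pawn (Trainkart) that respawns through BP_PlayerController when it gets stuck flipped over.
; Input axes drive throttle, steering and spring-arm camera rotation, and BeginPlay stores the start transform on the controller as RespawnLoco.
; Tick calls Flip, which tests up-vector tilt and low forward speed, then re-checks after a three-second Delay before destroying the actor.
; Destroyed calls the controller's Respawn.
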(event `self.ReceiveBeginPlay`
  (bind _asbp_player_controller (cast `/Game/KIA_Game/Game_BP/TimeTrial/BP_PlayerController` (`GameplayStatics.GetPlayerController` 0)))
  (bind _output_get (set `self.As BP Player Controller` _asbp_player_controller))
  (set `/Game/KIA_Game/Game_BP/TimeTrial/BP_PlayerController.RespawnLoco` (`self.GetTransform`) _output_get))

(event `InputAxis|Accelerate/reverse`
  (params (AxisValue :type "Float (single-precision)"))
  (`WheeledVehicleMovementComponent.SetThrottleInput` (`self.VehicleMovement`) AxisValue))

(event `InputAxis|Camera Control x`
  (params (AxisValue :type "Float (single-precision)"))
  (`SceneComponent.K2_AddRelativeRotation` (`self.SpringArm`) (`KismetMathLibrary.MakeRotator` 0.0 0.0 AxisValue) false false))

(event `InputAxis|Camera Control y`
  (params (AxisValue :type "Float (single-precision)"))
  (`SceneComponent.K2_AddRelativeRotation` (`self.SpringArm`) (`KismetMathLibrary.MakeRotator` 0.0 AxisValue) false false))

(event `InputAxis|Vehichle Steering`
  (params (AxisValue :type "Float (single-precision)"))
  (`WheeledVehicleMovementComponent.SetSteeringInput` (`self.VehicleMovement`) AxisValue))

(event `self.ReceiveTick`
  (params (DeltaSeconds :type "Float (single-precision)"))
  (bind _i_mstuck (`self.flip`))
  (if _i_mstuck
    (`KismetSystemLibrary.Delay` 3.0)
    (bind _i_mstuck_2 (`self.flip`))
    (if _i_mstuck_2
      (`self.K2_DestroyActor`))))

(event `self.ReceiveDestroyed`
  (`/Game/KIA_Game/Game_BP/TimeTrial/BP_PlayerController.Respawn` (`self.As BP Player Controller`)))

(fn `flip`
  (returns (`i'mStuck` :type Boolean))
  (if (and (< (`KismetMathLibrary.Dot_VectorVector` (`self.GetActorUpVector`) (0.0 0.0 1.0)) 0.5) (< (`WheeledVehicleMovementComponent.GetForwardSpeed` (`self.VehicleMovement`)) 0.5))
    (set `self.Stuck?` true)
    (else
      (set `self.Stuck?` false)))
  (return (`self.Stuck?`)))

(fn `UserConstructionScript`)